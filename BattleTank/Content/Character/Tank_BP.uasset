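; Player-controllable tank pawn Blueprint that wires input to its movement, aiming and camera components.
; BeginPlay initializes TankAiming with the barrel and turret, and TankMovement with both tracks.
; Forward and backward axes both feed IntendMoveForward, both track throttle axes feed IntendTurnRight, and Fire triggers TankAiming.
; Aim axes orbit the camera by yawing an azimuth gimbal and pitching the spring arm, scaled by delta time and sensitivity.
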(event `self.ReceiveBeginPlay`
  ;[1 1 1] Setup Meshes Reference
  (`|ExecutionSequence`
    (:`then_0`
      (`TankAimingComponent.Init` (`self.TankAiming`) (`self.Barrel`) (`self.Turret`)))
    (:`then_1`
      (`TankMovementComponent.Init` (`self.TankMovement`) (`self.Left Track`) (`self.Right Track`)))))

(event `InputAxis|Move Forward`
  (params (AxisValue :type "Float (single-precision)"))
  ;[1 1 1] Movement Input Binding
  (`TankMovementComponent.IntendMoveForward` (`self.TankMovement`) AxisValue))

(event `InputAxis|AimAzimuth`
  (params (AxisValue :type "Float (single-precision)"))
  ;[1 1 1] Caemra Input Binding (Axis X)
  (`SceneComponent.K2_AddLocalRotation` (`self.Azimuth Gimbal`) (`KismetMathLibrary.MakeRotator` 0.0 0.0 (* AxisValue (`GameplayStatics.GetWorldDeltaSeconds`) (`self.Sensitivity`))) false false))

(event `InputAxis|Move Backward`
  (params (AxisValue :type "Float (single-precision)"))
  ;[1 1 1] Movement Input Binding
  (`TankMovementComponent.IntendMoveForward` (`self.TankMovement`) AxisValue))

(event `InputAxis|Left Track Throttle`
  (params (AxisValue :type "Float (single-precision)"))
  ;[1 1 1] Movement Input Binding
  (`TankMovementComponent.IntendTurnRight` (`self.TankMovement`) AxisValue))

(event `InputAxis|AimElevation`
  (params (AxisValue :type "Float (single-precision)"))
  ;[1 1 1] Camera Input Binding (Axis Y)
  (`SceneComponent.K2_AddLocalRotation` (`self.SpringArm`) (`KismetMathLibrary.MakeRotator` 0.0 (* AxisValue (`GameplayStatics.GetWorldDeltaSeconds`) (`self.Sensitivity`))) false false))

(event `InputAxis|Right Track Throttle`
  (params (AxisValue :type "Float (single-precision)"))
  ;[1 1 1] Movement Input Binding
  (`TankMovementComponent.IntendTurnRight` (`self.TankMovement`) AxisValue))

(event `InputAction|Fire`
  (params (Key :type "Key Structure"))
  ;[1 1 1] Input Binding (Fire)
  (:`Pressed`
    (`TankAimingComponent.Fire` (`self.TankAiming`))))

(fn `UserConstructionScript`)